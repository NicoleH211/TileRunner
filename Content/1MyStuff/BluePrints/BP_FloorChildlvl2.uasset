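; BP_FloorChildlvl2 is a collapsing floor tile that vanishes after a BP_ThirdPersonCharacter overlaps its Box.
; The overlap shifts FloorMesh's Color through two timed warning stages using dynamic material instances, then disables actor collision and hides the mesh.
; It then reads TotalPlayers2 from PlayerTracker2, restoring collision, visibility and a pale color after a delay only when at least two players are counted.
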(event `self.Box.OnComponentBeginOverlap`
  (params (OverlappedComponent :type "PrimitiveComponent Object Reference") (OtherActor :type "Actor Object Reference") (OtherComp :type "PrimitiveComponent Object Reference") (OtherBodyIndex :type Integer) (bFromSweep :type Boolean) (SweepResult :type "HitResult Structure (by ref)"))
  (bind _floormesh (`self.floorMesh`))
  (bind _floormesh_2 (`self.floorMesh`))
  (cast `/Game/ThirdPerson/Blueprints/BP_ThirdPersonCharacter` OtherActor)
  (bind _returnvalue (`PrimitiveComponent.CreateDynamicMaterialInstance` (`self.floorMesh`) 0 null "None"))
  (`MaterialInstanceDynamic.SetVectorParameterValue` _returnvalue "Color" (make `LinearColor` 0.521 0.219 0.0 1.0))
  (`KismetSystemLibrary.Delay` 1.0)
  (bind _returnvalue_2 (`PrimitiveComponent.CreateDynamicMaterialInstance` _floormesh_2 0 null "None"))
  (`MaterialInstanceDynamic.SetVectorParameterValue` _returnvalue_2 "Color" (make `LinearColor` 0.693 0.0 0.0 1.0))
  (`KismetSystemLibrary.Delay` 1.0)
  (`self.SetActorEnableCollision` false)
  (`SceneComponent.SetVisibility` _floormesh_2 false false)
  (bind _returnvalue_3 (`GameplayStatics.GetActorOfClass` "/Game/1MyStuff/BluePrints/PlayerTracker2.PlayerTracker2_C"))
  (if (>= (`/Game/1MyStuff/BluePrints/PlayerTracker2.TotalPlayers2` _returnvalue_3) 2)
    (`KismetSystemLibrary.Delay` 3.0)
    (`self.SetActorEnableCollision` true)
    (`SceneComponent.SetVisibility` _floormesh true false)
    (bind _returnvalue_4 (`PrimitiveComponent.CreateDynamicMaterialInstance` _floormesh 0 null "None"))
    (`MaterialInstanceDynamic.SetVectorParameterValue` _returnvalue_4 "Color" (make `LinearColor` 0.8 0.8 0.65 1.0))))

(fn `UserConstructionScript`
  (`parent.UserConstructionScript`))