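; PlayerTracker3 is a trigger Blueprint that keeps a running count, TotalPlayers3, of what is inside its Box component.
; Begin overlap adds one and end overlap subtracts one, printing the new total each time.
; Neither event filters the overlapping actor, so any overlap changes the count despite the player-oriented name.
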(event `self.Box.OnComponentBeginOverlap`
  (params (OverlappedComponent :type "PrimitiveComponent Object Reference") (OtherActor :type "Actor Object Reference") (OtherComp :type "PrimitiveComponent Object Reference") (OtherBodyIndex :type Integer) (bFromSweep :type Boolean) (SweepResult :type "HitResult Structure (by ref)"))
  (bind _output_get (set `self.TotalPlayers3` (+ (`self.TotalPlayers3`) 1)))
  (`KismetSystemLibrary.PrintString` (`KismetStringLibrary.Conv_IntToString` _output_get)))

(event `self.Box.OnComponentEndOverlap`
  (params (OverlappedComponent :type "PrimitiveComponent Object Reference") (OtherActor :type "Actor Object Reference") (OtherComp :type "PrimitiveComponent Object Reference") (OtherBodyIndex :type Integer))
  (bind _output_get (set `self.TotalPlayers3` (- (`self.TotalPlayers3`) 1)))
  (`KismetSystemLibrary.PrintString` (`KismetStringLibrary.Conv_IntToString` _output_get)))

(fn `UserConstructionScript`
  (`parent.UserConstructionScript`))